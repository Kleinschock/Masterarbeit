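; Actor that imports a music file at runtime, plays it and analyzes it with Audio Analysis Tools to produce music-visualization values.
; Generated PCM data feeds the analyzer, which Tick polls for beat, kick, hi-hat, snare and spectral features, smoothed by running averages.
; FFT bands are averaged into overbands, normalized against decaying per-band maxima and buffered into VisArray.
; Older bass/mids/voice/highs scaling and debug drawing are disconnected.
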(event Custom|OnGeneratePCMData_Event
  (params (PCMData :type Array%20of%20Floats%20%28single-precision%29))
  ;[1 1 1] Get PCM Data
  (bind _audioframes (Class|AudioAnalysisToolsLibrary|GetAudiobyFrameSize (Variables|Default|GetAnalyzer) (stale Custom|OnResult_Event ImportedSoundWave) (Variables|Default|GetFrame%20Size)))
  (Class|AudioAnalysisToolsLibrary|ProcessAudioFrames (Variables|Default|GetAnalyzer) _audioframes true))

(event Custom|OnResult_Event
  (params (Importer :type Runtime%20Audio%20Importer%20Library%20Object%20Reference) (ImportedSoundWave :type Imported%20Sound%20Wave%20Object%20Reference) (Status :type ERuntimeImportStatus%20Enum :default "SuccessfulImport"))
  ;[0.1614 0.003472 0.1667] Load Soundwave File
  (Variables|Default|SetImporter Importer)
  (if (Utilities|Enum|Equal(Enum) Status "SuccessfulImport")
    (EventDispatchers|BindEventtoOnGeneratePCMData ImportedSoundWave (delegate Custom|OnGeneratePCMData_Event))
    (Audio|PlaySound2D ImportedSoundWave 1.0 1.0 0.0 0 0)))

(event EventBeginPlay
  (Utilities|FlowControl|Sequence
    (:then_0
      ;[0.1614 0.003472 0.1667] Load Soundwave File
      (bind _returnvalue (Class|RuntimeAudioImporterLibrary|CreateRuntimeAudioImporter))
      (bind _output_get (Variables|Default|SetImporter _returnvalue))
      (EventDispatchers|BindEventtoOnResult _output_get (delegate Custom|OnResult_Event))
      (Class|RuntimeAudioImporterLibrary|ImportAudiofromFile (Variables|Default|GetImporter) (Variables|Default|GetNew%20Sky) "Auto")
      (bind _returnvalue_2 (Class|AudioAnalysisToolsLibrary|CreateAudioAnalysisTools 4096 "BlackmanWindow"))
      (Variables|Default|SetAnalyzer _returnvalue_2)
      (Class|BeatDetection|UpdateFFTSubbandSize (Variables|/Script/AudioAnalysisTools.AudioAnalysisToolsLibrary|GetBeatDetection _returnvalue_2) (Variables|Default|GetFFT%20Subband%20Size)))))

(event Collision|EventActorBeginOverlap
  (params (OtherActor :type Actor%20Object%20Reference)))

(event EventTick
  (params (DeltaSeconds :type Float%20%28single-precision%29))
  (bind _analyzer (Variables|Default|GetAnalyzer))
  (Variables|Default|SetDelta%20Seconds DeltaSeconds)
  (Utilities|FlowControl|Sequence
    (:then_0
      ;[1 1 1] Get All Music Elements
      (Utilities|FlowControl|Sequence
        (:then_0
          (Variables|Default|SetisBeat%20Bool (Class|AudioAnalysisToolsLibrary|IsBeat _analyzer 7)))
        (:then_1
          (Variables|Default|SetisKick%20Bool (Class|BeatDetection|IsKick (Variables|/Script/AudioAnalysisTools.AudioAnalysisToolsLibrary|GetBeatDetection _analyzer))))
        (:then_2
          (Variables|Default|SetIs%20Hi%20Hat%20Bool (Class|AudioAnalysisToolsLibrary|IsHiHat _analyzer)))
        (:then_3
          (Variables|Default|SetIs%20Snare%20Bool (Class|AudioAnalysisToolsLibrary|IsSnare _analyzer)))))
    (:then_1)
    (:then_5
      (Utilities|FlowControl|Sequence
        (:then_0
          (bind _returnvalue (Class|AudioAnalysisToolsLibrary|GetRootMeanSquare (Variables|Default|GetAnalyzer)))
          (bind (_running_average _feature_value_array_output) (CallFunction|SimpleMean (Variables|Default|GetRootMeanSquare_Array) _returnvalue (Variables|Default|GetWindowSize)))
          (Variables|Default|SetRootMeanSquare_Array _feature_value_array_output)
          (Variables|Default|SetRoot%20Mean%20Square _running_average))
        (:then_1
          (bind _returnvalue_2 (Class|AudioAnalysisToolsLibrary|GetEnergyDifference (Variables|Default|GetAnalyzer)))
          (bind (_running_average_2 _feature_value_array_output_2) (CallFunction|SimpleMean (Variables|Default|GetEnergyDifference_Array) _returnvalue_2 (Variables|Default|GetWindowSize)))
          (Variables|Default|SetEnergyDifference_Array _feature_value_array_output_2)
          (Variables|Default|SetEnergy%20Difference _running_average_2))
        (:then_2
          (bind _returnvalue_3 (Class|AudioAnalysisToolsLibrary|GetSpectralCrest (Variables|Default|GetAnalyzer)))
          (bind (_running_average_3 _feature_value_array_output_3) (CallFunction|SimpleMean (Variables|Default|GetSpectralCrest_Array) _returnvalue_3 500))
          (Variables|Default|SetSpectralCrest_Array _feature_value_array_output_3)
          (Variables|Default|SetSpectral%20Crest _running_average_3))
        (:then_3
          (bind _returnvalue_4 (Class|AudioAnalysisToolsLibrary|GetSpectralCentroid (Variables|Default|GetAnalyzer)))
          (bind (_running_average_4 _feature_value_array_output_4) (CallFunction|SimpleMean (Variables|Default|GetSpectralCentroid_Array) _returnvalue_4 (Variables|Default|GetWindowSize)))
          (Variables|Default|SetSpectralCentroid_Array _feature_value_array_output_4)
          (Variables|Default|SetSpectral%20Centroid _running_average_4))
        (:then_4)
        (:then_5)
        (:then_6)
        (:then_7
          (bind _returnvalue_5 (Class|AudioAnalysisToolsLibrary|GetComplexSpectralDifference (Variables|Default|GetAnalyzer)))
          (bind (_running_average_5 _feature_value_array_output_5) (CallFunction|SimpleMean (Variables|Default|GetBand_CSD_Array) _returnvalue_5 (Variables|Default|GetWindowSize_400)))
          (Variables|Default|SetBand_CSD_Array _feature_value_array_output_5)
          (Variables|Default|SetCSD_Value _running_average_5))
        (:then_8
          (bind _returnvalue_6 (Class|AudioAnalysisToolsLibrary|GetZeroCrossingRate (Variables|Default|GetAnalyzer)))
          (bind (_running_average_6 _feature_value_array_output_6) (CallFunction|SimpleMean (Variables|Default|GetBand_ZeroCrossing_Array) _returnvalue_6 (Variables|Default|GetWindowSize_400)))
          (Variables|Default|SetZero%20Crossing _running_average_6)
          (Variables|Default|SetBand_ZeroCrossing_Array _feature_value_array_output_6))
        (:then_10
          (bind _returnvalue_7 (Class|AudioAnalysisToolsLibrary|GetHighFrequencyContent (Variables|Default|GetAnalyzer)))
          (bind (_running_average_7 _feature_value_array_output_7) (CallFunction|SimpleMean (Variables|Default|GetHighFrequencyCon_Array) _returnvalue_7 20))
          (bind _output_get (Variables|Default|SetHighFrequencyCon _running_average_7))
          (Variables|Default|SetHighFrequencyCon_Array _feature_value_array_output_7)
          (bind _newmax (CallFunction|DetectMaxBuffer&Decay _output_get (Variables|Default|GetHighFrequencyCon_Max) (Variables|Default|GetHFC_MAX_Buffer_decay)))
          (bind _output_get_2 (Variables|Default|SetHighFrequencyCon_Max _newmax))
          (Variables|Default|SetHighFrequencyCon (Math|Float|NormalizetoRange _output_get 0.0 _output_get_2))
          (Variables|Default|SetHighFrequencyCon_Max (- _output_get_2 (* (Variables|Default|GetHFC_MAX_Buffer_decay) (Variables|Default|GetDelta%20Seconds)))))
        (:then_11
          (bind _returnvalue_8 (Class|AudioAnalysisToolsLibrary|GetSpectralFlatness (Variables|Default|GetAnalyzer)))
          (bind (_running_average_8 _feature_value_array_output_8) (CallFunction|SimpleMean (Variables|Default|GetSpectralFlatness_Array) _returnvalue_8 5))
          (Variables|Default|SetSpectralFlatness_Array _feature_value_array_output_8)
          (Variables|Default|SetSpectralFlatness _running_average_8))
        (:then_12
          (Development|PrintString (Utilities|String|ToString(Float) (Class|AudioAnalysisToolsLibrary|GetBand (Variables|Default|GetAnalyzer) 59)))
          (bind _overbandarray_output (CallFunction|CreateOverbandsFixed (Variables|Default|GetOverbandSize)))
          (bind _maxarray_output (CallFunction|FindMax _overbandarray_output (Variables|Default|GetMax%20Array) (Variables|Default|GetDecay_Max)))
          (bind _visarray_output (CallFunction|Standatize _overbandarray_output _maxarray_output))
          (bind _buffer_array_output (CallFunction|GetBufferfromArray _visarray_output (Variables|Default|GetBuffer%20Array) (Variables|Default|GetDecay_Buffer)))
          (Variables|Default|SetVis%20Array _buffer_array_output))))))

(fn ConstructionScript)

(fn CountAttribute
  (params (Decay :type Float%20%28double-precision%29) (Value :type Integer) (Condition :type Boolean))
  (bind _returnvalue (Utilities|Text|ToText(Integer) Value))
  (if Condition
    (Development|PrintString "Hello")
    (return _returnvalue)
    (else
      (Variables|Default|SetBeat%20counter (+ 1 Decay))
      (Development|PrintText _returnvalue)
      (Variables|Default|SetKickCounted true))))

(fn SimpleMean
  (params (Feature%20Value%20Array :type Array%20of%20Floats%20%28double-precision%29) (Feature%20Value :type Float%20%28double-precision%29) (WindowSize :type Integer))
  (bind _returnvalue (Utilities|Array|Add Feature%20Value%20Array Feature%20Value))
  (if (>= _returnvalue WindowSize)
    (Utilities|Array|RemoveIndex Feature%20Value%20Array))
  (for (_array_element _array_index) Feature%20Value%20Array
    (LocalVariables|SetArraySum (+ _array_element (LocalVariables|GetArraySum))))
  (return (/ (LocalVariables|GetArraySum) (+ _array_index 1)) Feature%20Value%20Array))

(fn DecayingMean
  (params (Feature%20Value%20Array :type Array%20of%20Floats%20%28double-precision%29) (Feature%20Value :type Float%20%28double-precision%29) (WindowSize :type Integer) (Weight :type Float%20%28double-precision%29))
  (bind _returnvalue (Utilities|Array|Add Feature%20Value%20Array Feature%20Value))
  (if (>= _returnvalue WindowSize)
    (Utilities|Array|RemoveIndex Feature%20Value%20Array))
  (for (_array_element _array_index) Feature%20Value%20Array
    (LocalVariables|SetFloatSave (+ _array_element (LocalVariables|GetFloatSave))))
  (return (/ (LocalVariables|GetFloatSave) (+ _array_index 1)) Feature%20Value%20Array))

(fn GetBandsinRange
  (params (StartBand :type Integer) (EndBand :type Integer))
  (for _index (range StartBand EndBand)
    (LocalVariables|SetBandSum (+ (Class|AudioAnalysisToolsLibrary|GetBand (Variables|Default|GetAnalyzer) (Class|KismetMathLibrary|ToInt64(Integer) _index)) (LocalVariables|GetBandSum))))
  (return (/ (LocalVariables|GetBandSum) (- EndBand StartBand))))

(fn DetectMaxBuffer&Decay
  (params (CurrentValue :type Float%20%28double-precision%29) (CurrentMax :type Float%20%28double-precision%29) (Decay :type Float%20%28double-precision%29))
  (bind _delta_seconds (Variables|Default|GetDelta%20Seconds))
  (bind _returnvalue (* CurrentMax Decay _delta_seconds))
  (if (> (- CurrentValue _returnvalue) CurrentMax)
    (LocalVariables|SetNew%20Max CurrentValue)
    (else
      (LocalVariables|SetNew%20Max CurrentMax)))
  (return (- (LocalVariables|GetNew%20Max) _returnvalue)))

(fn GetBandArray
  (for _index (range 0 (Math|Conversions|ToInteger(Byte) (Variables|Default|GetFFT%20Subband%20Size)))
    (Utilities|Array|SetArrayElem (LocalVariables|Getm_Band_Array) _index (Class|AudioAnalysisToolsLibrary|GetBand (Variables|Default|GetAnalyzer) (Class|KismetMathLibrary|ToInt64(Integer) _index)) true)
    (if (> (Class|AudioAnalysisToolsLibrary|GetBand (Variables|Default|GetAnalyzer) (Class|KismetMathLibrary|ToInt64(Integer) _index)) 0.0)
      (Development|PrintString "Hello")))
  (return (LocalVariables|Getm_Band_Array)))

(fn GetBufferfromArray
  (params (Band_Array :type Array%20of%20Floats%20%28double-precision%29) (Buffer_Array :type Array%20of%20Floats%20%28double-precision%29) (Decay :type Float%20%28double-precision%29))
  (for (_array_element _array_index) Band_Array
    (if (>= (- _array_element (* _array_element Decay (Variables|Default|GetDelta%20Seconds))) (Utilities|Array|Get(acopy) Buffer_Array _array_index))
      (Utilities|Array|SetArrayElem Buffer_Array _array_index _array_element true)
      (else
        (Utilities|Array|SetArrayElem Buffer_Array _array_index (- _array_element (* _array_element Decay (Variables|Default|GetDelta%20Seconds))) true))))
  (return Buffer_Array))

(fn FindMax
  (params (BandArray :type Array%20of%20Floats%20%28double-precision%29) (MaxArray :type Array%20of%20Floats%20%28double-precision%29) (Decay :type Float%20%28double-precision%29))
  (for (_array_element _array_index) BandArray
    (if (> _array_element (Utilities|Array|Get(acopy) MaxArray _array_index))
      (Utilities|Array|SetArrayElem MaxArray _array_index _array_element true)
      (else
        (Utilities|Array|SetArrayElem MaxArray _array_index (- (Utilities|Array|Get(acopy) MaxArray _array_index) (* Decay (Variables|Default|GetDelta%20Seconds) (Utilities|Array|Get(acopy) MaxArray _array_index))) true))))
  (return MaxArray))

(fn Standatize
  (params (BufferArray :type Array%20of%20Floats%20%28double-precision%29) (MaxArray :type Array%20of%20Floats%20%28double-precision%29))
  (for (_array_element _array_index) BufferArray
    (Utilities|Array|SetArrayElem (LocalVariables|GetVisArray) _array_index (/ _array_element (Utilities|Array|Get(acopy) MaxArray _array_index)) true))
  (return (LocalVariables|GetVisArray)))

(fn MapSubbandstoOverbands
  (params (total%20overband%20size :type Float%20%28double-precision%29))
  (LocalVariables|SetFrequency%20per%20subband (/ (Variables|Default|GetVis_Hz) (Variables|Default|GetFFT%20Subband%20Size)))
  (for _index (range 0 (- (Math|Conversions|ToInteger(Byte) (Variables|Default|GetFFT%20Subband%20Size)) 1))
    (Utilities|FlowControl|Sequence
      (:then_0
        (if (not (> (|(log(x)) (Math|Conversions|ToFloat(Integer) _index)) (Variables|Default|GetVis_Hz)))
          (Utilities|Array|SetArrayElem (LocalVariables|Getoverband%20eckpunkte) _index (|(log(x)) (Math|Conversions|ToFloat(Integer) _index)) true))))))

(fn LogarithmicOverbandEdges
  (params (maxfreq :type Float%20%28double-precision%29) (overbands :type Array%20of%20Floats%20%28double-precision%29)))

(fn CreateOverbands
  (params (BandArray :type Array%20of%20Floats%20%28double-precision%29) (OverbandSize :type Array%20of%20Integers))
  (for _index (range 0 (- (Utilities|Array|Length OverbandSize) 1))
    (if (== _index 0)
      (LocalVariables|SetisZero? 0)
      (else
        (LocalVariables|SetisZero? 1)))
    (for _index_2 (range (Utilities|Array|Get(acopy) OverbandSize (- _index (LocalVariables|GetisZero?))) (Utilities|Array|Get(acopy) OverbandSize _index))
      (LocalVariables|SetBandSum (+ (Utilities|Array|Get(acopy) BandArray _index_2) (LocalVariables|GetBandSum))))
    (Utilities|Array|SetArrayElem (LocalVariables|Getm_OverbandArray) _index (/ (LocalVariables|GetBandSum) (Utilities|Operators|Subtract (Utilities|Array|Get(acopy) OverbandSize _index) (Utilities|Array|Get(acopy) OverbandSize (- _index (LocalVariables|GetisZero?))) (LocalVariables|GetNewLocalVar_0))) true))
  (return (LocalVariables|Getm_OverbandArray)))

(fn CreateOverbandsFixed
  (params (OverbandSize :type Array%20of%20Integers))
  (for (_array_element _array_index) OverbandSize
    (bind _bandaverage (CallFunction|GetBandsinRange (LocalVariables|Getprevious%20Bandrange) (+ (LocalVariables|Getprevious%20Bandrange) _array_element)))
    (LocalVariables|Setprevious%20Bandrange (+ (LocalVariables|Getprevious%20Bandrange) _array_element))
    (Utilities|Array|SetArrayElem (LocalVariables|Getm_OverbandArray_Output) _array_index _bandaverage true))
  (return (LocalVariables|Getm_OverbandArray_Output)))

(fn ArrayMean
  (params (Feature%20Value%20Array :type Array%20of%20Floats%20%28double-precision%29) (Feature%20Value :type Float%20%28double-precision%29) (WindowSize :type Integer))
  (bind _returnvalue (Utilities|Array|Add Feature%20Value%20Array Feature%20Value))
  (if (>= _returnvalue WindowSize)
    (Utilities|Array|RemoveIndex Feature%20Value%20Array))
  (for (_array_element _array_index) Feature%20Value%20Array
    (LocalVariables|SetArraySum (+ _array_element (LocalVariables|GetArraySum))))
  (return (/ (LocalVariables|GetArraySum) (+ _array_index 1)) Feature%20Value%20Array))