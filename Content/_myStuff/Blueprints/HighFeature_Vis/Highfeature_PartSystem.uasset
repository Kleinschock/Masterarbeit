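; Audio visualizer actor that drives a Fireflies Niagara particle system from live audio analysis values.
; The construction script finds the AudioAnaly_Plugin_HF actor in the level and stores it as VisMaster, keeping the last one found.
; Every tick it copies VisMaster's loudness, spectral, frequency band and kick detection values into the Niagara system's float parameters, converting the kick boolean to a float.
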(event `self.ReceiveTick`
  (params (DeltaSeconds :type "Float (single-precision)"))
  (bind _vis_master (`self.Vis_Master`))
  (bind _fireflies (`self.Fireflies`))
  (bind _fireflies_2 (`self.Fireflies`))
  (`NiagaraComponent.SetVariableFloat` (`self.Fireflies`) "Visualizer_RootSquare" (`/Game/_myStuff/Blueprints/HighFeature_Vis/audioAnaly_Plugin_HF.Root Mean Square` _vis_master))
  (`NiagaraComponent.SetVariableFloat` (`self.Fireflies`) "Visualizer_Crest" (`/Game/_myStuff/Blueprints/HighFeature_Vis/audioAnaly_Plugin_HF.Spectral Crest` _vis_master))
  (`NiagaraComponent.SetVariableFloat` (`self.Fireflies`) "Visualizer_Zero" (`/Game/_myStuff/Blueprints/HighFeature_Vis/audioAnaly_Plugin_HF.Zero Crossing` _vis_master))
  (`NiagaraComponent.SetVariableFloat` (`self.Fireflies`) "Visualizer_Complex" (`/Game/_myStuff/Blueprints/HighFeature_Vis/audioAnaly_Plugin_HF.CSD_Value` _vis_master))
  (`NiagaraComponent.SetVariableFloat` (`self.Fireflies`) "Visualizer_Band_Bass" (`/Game/_myStuff/Blueprints/HighFeature_Vis/audioAnaly_Plugin_HF.Band Bass` _vis_master))
  (`NiagaraComponent.SetVariableFloat` (`self.Fireflies`) "Visualizer_Band_Mids" (`/Game/_myStuff/Blueprints/HighFeature_Vis/audioAnaly_Plugin_HF.Band_Mids` _vis_master))
  (`NiagaraComponent.SetVariableFloat` _fireflies_2 "Visualizer_Band_Voice" (`/Game/_myStuff/Blueprints/HighFeature_Vis/audioAnaly_Plugin_HF.Band_Voice` _vis_master))
  (`NiagaraComponent.SetNiagaraVariableFloat` _fireflies_2 "Visualizer_isKickFloat" (`KismetMathLibrary.Conv_BoolToDouble` (`/Game/_myStuff/Blueprints/HighFeature_Vis/audioAnaly_Plugin_HF.isKick Bool` _vis_master)))
  (`NiagaraComponent.SetNiagaraVariableFloat` _fireflies "Visualizer_Band_Highs" (`/Game/_myStuff/Blueprints/HighFeature_Vis/audioAnaly_Plugin_HF.Band_Highs` _vis_master))
  (`NiagaraComponent.SetNiagaraVariableFloat` _fireflies "Visualizer_EnergyDifference" (`/Game/_myStuff/Blueprints/HighFeature_Vis/audioAnaly_Plugin_HF.Energy Difference` _vis_master))
  (`NiagaraComponent.SetNiagaraVariableFloat` _fireflies "Visualizer_HighFrequencyCon" (`/Game/_myStuff/Blueprints/HighFeature_Vis/audioAnaly_Plugin_HF.HighFrequencyCon` _vis_master))
  (`NiagaraComponent.SetNiagaraVariableFloat` _fireflies "Visualizer_Flatness" (`/Game/_myStuff/Blueprints/HighFeature_Vis/audioAnaly_Plugin_HF.SpectralFlatness` _vis_master))
  (`NiagaraComponent.SetNiagaraVariableFloat` _fireflies "Visualizer_Centroid" (`/Game/_myStuff/Blueprints/HighFeature_Vis/audioAnaly_Plugin_HF.Spectral Centroid` _vis_master)))

(fn `UserConstructionScript`
  (bind _outactors (`GameplayStatics.GetAllActorsOfClass` "/Game/_myStuff/Blueprints/HighFeature_Vis/audioAnaly_Plugin_HF.audioAnaly_Plugin_HF_C"))
  (for _array_element _outactors
    (set `self.Vis_Master` _array_element)))