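; BP_StudyGameController is a controller for a VR/AR study with firefly visualizers and SAM ratings.
; On BeginPlay it caches both hand firefly actors and reads BP_StudyManager's condition to set floor visualizer intensity, also hiding the VRPawn's hands in AR.
; Helper functions activate the audio analysis and firefly actors or reset the last valence, arousal and dominance scores.
; SetPassthroughMode is an empty stub.
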(event `self.ReceiveBeginPlay`
  (bind _returnvalue (`GameplayStatics.GetActorOfClass` "/Game/_myStuff/Blueprints/ParticleVis/Firefly_Right.Firefly_Right_C"))
  (set `self.m_Firefly_Hand_Right` _returnvalue)
  (bind _returnvalue_2 (`GameplayStatics.GetActorOfClass` "/Game/_myStuff/Blueprints/ParticleVis/Firefly_Left.Firefly_Left_C"))
  (set `self.m_Firefly_Hand_Left` _returnvalue_2)
  (bind _returnvalue_3 (`GameplayStatics.GetActorOfClass` "/Game/_myStuff/UI/BP_StudyManager.BP_StudyManager_C"))
  (switch `EBetweenCondition` (`StudyManager.BetweenCondition` _returnvalue_3)
    (:`VR`
      (bind _returnvalue_4 (`GameplayStatics.GetActorOfClass` "/Game/_myStuff/Blueprints/ParticleVis/Firefly_Floor.Firefly_Floor_C"))
      (set `/Game/_myStuff/Blueprints/ParticleVis/Firefly_Floor.Visualizer_Color_Intensity_Floor` 0.5 _returnvalue_4))
    (:`AR`
      (bind _returnvalue_5 (`GameplayStatics.GetActorOfClass` "/Game/_myStuff/Blueprints/ParticleVis/Firefly_Floor.Firefly_Floor_C"))
      (set `/Game/_myStuff/Blueprints/ParticleVis/Firefly_Floor.Visualizer_Color_Intensity_Floor` 0.8 _returnvalue_5)
      (bind _returnvalue_6 (`GameplayStatics.GetActorOfClass` "/Game/VRTemplate/Blueprints/VRPawn.VRPawn_C"))
      (`SceneComponent.SetVisibility` (`/Game/VRTemplate/Blueprints/VRPawn.HandRight` _returnvalue_6) false false)
      (`SceneComponent.SetVisibility` (`/Game/VRTemplate/Blueprints/VRPawn.HandLeft` _returnvalue_6) false false)
      (`KismetSystemLibrary.PrintString` "AR MODE ACTIVATED"))))

(event `self.SetPassthroughMode`
  (params (bEnable :type Boolean))
  (if bEnable
    _))

(fn `ActivateObject`
  (params (Actor :type "Actor Object Reference"))
  (`self.SetActorHiddenInGame` Actor false)
  (`self.SetActorTickEnabled` Actor true))

(fn `ActivateObjectAndCollision`
  (params (Actor :type "Actor Object Reference"))
  (`self.SetActorHiddenInGame` Actor false)
  (`self.SetActorTickEnabled` Actor true)
  (`self.SetActorEnableCollision` Actor true))

(fn `ActivateObjectsForVis`
  (`self.ActivateObject` (`self.m_AudioAnalysis`))
  (`KismetSystemLibrary.PrintString` "DEBUG | BP_Mainmenu: Audio Analysis Blueprint was activated.")
  (`self.ActivateObject` (`self.m_Firefly`))
  (`KismetSystemLibrary.PrintString` "DEBUG | BP_Mainmenu: Firefly (normal) was activated.")
  (`self.ActivateObject` (`self.m_Firefly_Hand_Left`))
  (`self.ActivateObject` (`self.m_Firefly_Hand_Right`))
  (`KismetSystemLibrary.PrintString` "DEBUG | BP_Mainmenu: Firefly (Hand) was activated."))

(fn `ResetLastScore`
  (set `self.m_lastValence` 0)
  (set `self.m_lastArousal` 0)
  (set `self.m_lastDominance` 0)
  (`KismetSystemLibrary.PrintString` "DEBUG | BP_StudyGameController: The last values of SAM have been reset."))

(fn `UserConstructionScript`)