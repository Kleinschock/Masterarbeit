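; Right-hand firefly Niagara actor for a VR audio-visualization study, activated while the right grab is held.
; During tutorial, running and fade-out phases, Tick feeds it audio features from AudioAnaly_Plugin, or defaults in tutorials.
; It also passes pawn, camera, current and previous hand positions, plus controller inputs, which are zeroed outside tutorial or interaction conditions.
; The study controller's phase drives an Experiment_Fader that ramps down during fade-out.
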(event `self.ReceiveBeginPlay`
  (bind _returnvalue (`GameplayStatics.GetActorOfClass` "/Game/VRTemplate/Blueprints/VRPawn.VRPawn_C"))
  (set `self.VR_PAWN` _returnvalue)
  (set `self.niagaraObject` (`self.Fireflies`))
  (set `self.isInitialized` true)
  (bind _returnvalue_2 (`GameplayStatics.GetActorOfClass` "/Game/_myStuff/Blueprints/BP_StudyGameController.BP_StudyGameController_C"))
  (set `self.m_BP_StudyGameController` _returnvalue_2)
  (`KismetSystemLibrary.PrintString` "DEBUG | Firefly: Is inisitalized"))

(event `self.ReceiveTick`
  (params (DeltaSeconds :type "Float (single-precision)"))
  (bind _fireflies (`self.Fireflies`))
  (bind _m_bp_studygamecontroller (`self.m_BP_StudyGameController`))
  (bind _vis_master (`self.Vis_Master`))
  (bind _vr_pawn (`self.VR_PAWN`))
  (bind _returnvalue (`SceneComponent.K2_GetComponentLocation` (`/Game/VRTemplate/Blueprints/VRPawn.XRDeviceVisualizationLeft` _vr_pawn)))
  (bind _returnvalue_2 (`SceneComponent.K2_GetComponentLocation` (`/Game/VRTemplate/Blueprints/VRPawn.XRDeviceVisualizationRight` _vr_pawn)))
  (if (`self.isInitialized`)
    (switch `EStudyPhase` (`StudyGameController.CurrentPhase` (`self.m_BP_StudyGameController`))
      (:`GeneralTutorial`
        _)
      (:`InteractionTutorial`
        _)
      (:`Running`
        _)
      (:`FadingOut`
        _))
    (`|ExecutionSequence`
      (:`then_0`
        (switch `EStudyPhase` (`StudyGameController.CurrentPhase` (`self.m_BP_StudyGameController`))
          (:`GeneralTutorial`
            (`self.SetVisValues` (`self.Fireflies`) (`self.default_RootSquare`) (`self.default_Crest`) (`self.default_Zero`) (`self.default_Complex`) (`self.particleSize`) (`self.default_CSD`) (`self.maxDistance`) (`self.default_Centroid`) (`self.default_Flatness`) (`self.default_EnergyDifference`) (`self.default_Band_Array`) :!label _label))
          (:`InteractionTutorial`
            (goto _label))
          (:`Running`
            (`self.SetVisValues` (`self.Fireflies`) (`/Game/_myStuff/Blueprints/ParticleVis/audioAnaly_Plugin.Root Mean Square` _vis_master) (`/Game/_myStuff/Blueprints/ParticleVis/audioAnaly_Plugin.Spectral Crest` _vis_master) (`/Game/_myStuff/Blueprints/ParticleVis/audioAnaly_Plugin.Zero Crossing` _vis_master) (`/Game/_myStuff/Blueprints/ParticleVis/audioAnaly_Plugin.CSD_Value` _vis_master) (`self.particleSize`) (`/Game/_myStuff/Blueprints/ParticleVis/audioAnaly_Plugin.CSD_Value` _vis_master) (`self.maxDistance`) (`/Game/_myStuff/Blueprints/ParticleVis/audioAnaly_Plugin.SpectralCentroid` _vis_master) (`/Game/_myStuff/Blueprints/ParticleVis/audioAnaly_Plugin.SpectralFlatness` _vis_master) (`/Game/_myStuff/Blueprints/ParticleVis/audioAnaly_Plugin.Energy Difference` _vis_master) (`/Game/_myStuff/Blueprints/ParticleVis/audioAnaly_Plugin.Vis Array` _vis_master) :!label _label_2))
          (:`FadingOut`
            (goto _label_2))))
      (:`then_1`
        (`NiagaraComponent.SetNiagaraVariableVec3` _fireflies "Interaction_Right_Position" _returnvalue_2)
        (bind _output_get (set `self.prev_Interaction_Right_Position` (`self.Position_Hand_Right`)))
        (set `self.Position_Hand_Right` _returnvalue_2)
        (`NiagaraComponent.SetNiagaraVariableVec3` _fireflies "prev_Interaction_Right_Position" _output_get)
        (`NiagaraComponent.SetNiagaraVariableVec3` _fireflies "Interaction_Left_Position" _returnvalue)
        (bind _output_get_2 (set `self.prev_Interaction_Left_Position` (`self.Position_Hand_Left`)))
        (set `self.Position_Hand_Left` _returnvalue)
        (`NiagaraComponent.SetNiagaraVariableVec3` _fireflies "prev_Interaction_Left_Position" _output_get_2)
        (if (or (`self.isInteraction`) (`self.IsTutorial`))
          (`self.SetControllerValues` _fireflies (`/Game/VRTemplate/Blueprints/VRPawn.Left_Grab` _vr_pawn) (`/Game/VRTemplate/Blueprints/VRPawn.Left_Trigger` _vr_pawn) (`/Game/VRTemplate/Blueprints/VRPawn.Right_Grab` _vr_pawn) (`/Game/VRTemplate/Blueprints/VRPawn.Right_Trigger` _vr_pawn))
          (else
            (`self.SetControllerValues` _fireflies)
            (`self.SetInteractionZero` _vr_pawn)))
        (`self.ActivateDeactivateHand` (`/Game/VRTemplate/Blueprints/VRPawn.Right_Grab` _vr_pawn))
        (`NiagaraComponent.SetNiagaraVariableVec3` _fireflies "Interaction_Pawn" (`SceneComponent.K2_GetComponentLocation` (`/Game/VRTemplate/Blueprints/VRPawn.VROrigin` _vr_pawn)))
        (`NiagaraComponent.SetNiagaraVariableVec3` _fireflies "Interaction_Camera" (`SceneComponent.K2_GetComponentLocation` (`/Game/VRTemplate/Blueprints/VRPawn.Camera` _vr_pawn)))
        (switch `EStudyPhase` (`StudyGameController.CurrentPhase` _m_bp_studygamecontroller)
          (:`MainMenu`
            (`NiagaraComponent.SetVariableFloat` _fireflies "Experiment_Fader" 0.0 :!label _label_3))
          (:`GeneralTutorial`
            (goto _label_3))
          (:`InteractionTutorial`
            (`NiagaraComponent.SetVariableFloat` _fireflies "Experiment_Fader" 1.0 :!label _label_4))
          (:`Briefing`
            (goto _label_3))
          (:`Preparation`
            (goto _label_3))
          (:`Running`
            (goto _label_4))
          (:`FadingOut`
            (`NiagaraComponent.SetVariableFloat` _fireflies "Experiment_Fader" (/ (`StudyGameController.CurrentFadeOutTimeRemaining` _m_bp_studygamecontroller) (`StudyGameController.FadeOutDuration` _m_bp_studygamecontroller))))
          (:`SamEvaluation`
            (goto _label_3))
          (:`PresenceEvaluation`
            (goto _label_3))
          (:`Complete`
            (goto _label_3)))))
    (else
      (`KismetSystemLibrary.PrintString` "FIREFLY Hello"))))

(event `self.StartVisualization_ControlOnly`
  (`KismetSystemLibrary.PrintString` "EVENT Start Vis Control Only: Tutorial Vis Started. VIs Values are not used.")
  (set `self.isExperiment` false)
  (set `self.IsTutorial` true)
  (set `self.isInteraction` false)
  (set `self.isControl` false))

(event `self.StopActiveVisualization`
  (`KismetSystemLibrary.PrintString` "EVENT STOP ACTIVE VIS: Visualization Stopped")
  (set `self.isExperiment` false)
  (set `self.IsTutorial` false)
  (set `self.isInteraction` false)
  (set `self.isControl` false))

(event `self.StartActiveVisualization`
  (params (CurrentCondition :type "EConditionType Enum" :default "Control"))
  (switch `EConditionType` CurrentCondition
    (:`Control`
      (set `self.isControl` true)
      (set `self.isInteraction` false))
    (:`NoInteraction`
      (set `self.isInteraction` false)
      (set `self.isControl` false))
    (:`WithInteraction`
      (set `self.isInteraction` true)
      (set `self.isControl` false)))
  (set `self.isExperiment` true)
  (set `self.IsTutorial` false))

(fn `ActivateDeactivateHand`
  (params (InteractionTrigger :type Boolean))
  (bind _fireflies (`self.Fireflies`))
  (if InteractionTrigger
    (if (not (`self.isActive`))
      (`ActorComponent.Activate` _fireflies false)
      (set `self.isActive` true))
    (else
      (`ActorComponent.Deactivate` _fireflies)
      (set `self.isActive` false))))

(fn `SetControllerValues`
  (params (NiagaraParticleSystem :type "NiagaraComponent Object Reference") (Interaction_Left_Grab :type Boolean) (Interaction_Left_Trigger :type Boolean) (Interaction_Right_Grab :type Boolean) (Interaction_Right_Trigger :type Boolean))
  (`|ExecutionSequence`
    (:`then_0`
      (`NiagaraComponent.SetNiagaraVariableBool` NiagaraParticleSystem "Interaction_Left_Grab" Interaction_Left_Grab))
    (:`then_1`
      (`NiagaraComponent.SetNiagaraVariableBool` NiagaraParticleSystem "Interaction_Left_Trigger" Interaction_Left_Trigger))
    (:`then_2`
      (`NiagaraComponent.SetNiagaraVariableBool` NiagaraParticleSystem "Interaction_Right_Grab" Interaction_Right_Grab))
    (:`then_3`
      (`NiagaraComponent.SetNiagaraVariableBool` NiagaraParticleSystem "Interaction_Right_Trigger" Interaction_Right_Trigger))))

(fn `SetInteractionZero`
  (params (VRPawn :type "/Game/VRTemplate/Blueprints/VRPawn Object Reference"))
  (set `/Game/VRTemplate/Blueprints/VRPawn.Left_Grab` false VRPawn)
  (set `/Game/VRTemplate/Blueprints/VRPawn.Right_Grab` false VRPawn)
  (set `/Game/VRTemplate/Blueprints/VRPawn.Left_Trigger` false VRPawn)
  (set `/Game/VRTemplate/Blueprints/VRPawn.Right_Trigger` false VRPawn))

(fn `SetVisValues`
  (params (NiagaraSystem :type "NiagaraComponent Object Reference") (RootSquare :type "Float (single-precision)") (Crest :type "Float (single-precision)") (Zero :type "Float (single-precision)") (Complex :type "Float (single-precision)") (particleSize :type "Float (single-precision)") (CSD :type "Float (single-precision)") (maxDistance :type "Float (single-precision)") (Centroid :type "Float (single-precision)") (Flatness :type "Float (single-precision)") (EnergyDifference :type "Float (single-precision)") (Band_Array :type "Array of Float (single-precision) (by ref)"))
  (`|ExecutionSequence`
    (:`then_0`
      (`NiagaraComponent.SetVariableFloat` NiagaraSystem "Visualizer_RootSquare" RootSquare))
    (:`then_1`
      (`NiagaraComponent.SetVariableFloat` NiagaraSystem "Visualizer_Crest" Crest))
    (:`then_2`
      (`NiagaraComponent.SetVariableFloat` NiagaraSystem "Visualizer_Zero" Zero))
    (:`then_3`
      (`NiagaraComponent.SetVariableFloat` NiagaraSystem "Visualizer_Complex" Complex))
    (:`then_4`
      (`NiagaraComponent.SetNiagaraVariableFloat` NiagaraSystem "Visualizer_particleSize" particleSize))
    (:`then_5`
      (`NiagaraComponent.SetNiagaraVariableFloat` NiagaraSystem "Visualizer_CSD_Value" CSD))
    (:`then_6`
      (`NiagaraComponent.SetNiagaraVariableFloat` NiagaraSystem "Visualizer_maxDistance" maxDistance))
    (:`then_7`
      (`NiagaraComponent.SetNiagaraVariableFloat` NiagaraSystem "Visualizer_Centroid" Centroid))
    (:`then_8`
      (`NiagaraComponent.SetNiagaraVariableFloat` NiagaraSystem "Visualizer_Flatness" Flatness))
    (:`then_9`
      (`NiagaraComponent.SetNiagaraVariableFloat` NiagaraSystem "Visualizer_EnergyDifference" EnergyDifference))
    (:`then_10`
      (`NiagaraDataInterfaceArrayFunctionLibrary.SetNiagaraArrayFloat` NiagaraSystem "Visualizer_Band_Array" Band_Array))))

(fn `UserConstructionScript`
  (bind _outactors (`GameplayStatics.GetAllActorsOfClass` "/Game/_myStuff/Blueprints/ParticleVis/audioAnaly_Plugin.audioAnaly_Plugin_C"))
  (for _array_element _outactors
    (set `self.Vis_Master` _array_element)))