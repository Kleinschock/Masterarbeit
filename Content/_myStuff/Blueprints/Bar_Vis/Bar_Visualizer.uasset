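; Actor that draws an audio visualizer as a row of bars driven by an AudioAnaly_Plugin_Bar actor in the level.
; On BeginPlay it spawns one bar per OverbandSize entry along the world right axis, using the class of a Bar_Single found in the level.
; Each Tick sets every bar's uniform scale from its VisArray value, IntensityScale and DeltaSeconds, so size varies with frame rate.
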(event `self.ReceiveBeginPlay`
  (bind _returnvalue (`GameplayStatics.GetActorOfClass` "/Game/_myStuff/Blueprints/ParticleVis/OLD/audioAnaly_Plugin_Bar.audioAnaly_Plugin_Bar_C"))
  (set `self.Audio_Analyser` _returnvalue)
  (bind _returnvalue_2 (`GameplayStatics.GetActorOfClass` "/Game/_myStuff/Blueprints/Bar_Vis/Bar_Single.Bar_Single_C"))
  (set `self.Bar_Single_Object` _returnvalue_2)
  (for _index (range (`KismetArrayLibrary.Array_Length` (`/Game/_myStuff/Blueprints/ParticleVis/OLD/audioAnaly_Plugin_Bar.OverbandSize` (`self.Audio_Analyser`))))
    (bind _returnvalue_3 (`|SpawnActorFromClass` (`GameplayStatics.GetObjectClass` (`self.Bar_Single_Object`)) (`KismetMathLibrary.MakeTransform` (+ (* _index (`self.bar_single_distance`) (`KismetMathLibrary.Vector_Right`)) (`self.K2_GetActorLocation` self)) (struct :`Pitch` 1.0)) "Undefined" "MultiplyWithRoot" null null))
    (`KismetArrayLibrary.Array_Set` (`self.Bar_Array`) _index _returnvalue_3 true)))

(event `self.ReceiveTick`
  (params (DeltaSeconds :type "Float (single-precision)"))
  (set `self.Delta Seconds` DeltaSeconds)
  (for (_array_element _array_index) (`self.Bar_Array`)
    (`self.SetActorScale3D` _array_element (* (`|GetArrayItem` (`/Game/_myStuff/Blueprints/ParticleVis/OLD/audioAnaly_Plugin_Bar.Vis Array` (`self.Audio_Analyser`)) _array_index) (1.0 1.0 1.0) (`self.Delta Seconds`) (`self.intensity_scale`)))))

(fn `UserConstructionScript`)